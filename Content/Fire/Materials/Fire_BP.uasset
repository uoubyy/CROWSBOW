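; Fire effect actor that keeps itself turned toward the player camera as a yaw-only billboard.
; A looping timer started on BeginPlay calls GetAngle, which flattens the camera direction to the horizontal plane and sets the actor rotation from it.
; BeginPlay also plays a LightFlicker timeline, but the node that sets point light intensity is unconnected and never runs.
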(event EventBeginPlay
  (Utilities|Time|SetTimerbyFunctionName 0 "GetAngle" 0.1 true)
  (Timeline|Light%20Flicker Play))

(fn ConstructionScript)

(fn GetAngle
  (Transformation|SetActorRotation (Math|Conversions|RotationFromXVector (Math|Vector|Normalize (* (- (Camera|GetCameraLocation (Game|GetPlayerCameraManager 0)) (Transformation|GetActorLocation)) "1.000000,1.000000, 0")))))