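; BP_Boss is the boss enemy in EndlessGraves, adding an idle back-and-forth rotation around Z.
; While the enemy state is Idle, Tick advances CurZ by delta time and flips Direction at MinZ and MaxZ.
; CurZ is written to ZRotation on the ABP_Boss anim instance, so the animation Blueprint receives the sweep.
; GetRotationAroundZ simply returns the value from GetRotationZ.
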(event EventBeginPlay)

(event Collision|EventActorBeginOverlap
  (params (OtherActor :type Actor%20Object%20Reference)))

(event EventTick
  (params (DeltaSeconds :type Float%20%28single-precision%29))
  (if (Utilities|Enum|Equal(Enum) (Class|EndlessGravesAICharacter|GetEnemyState) "ES_Idle")
    (bind _output_get (Variables|Default|SetCurZ (+ (Variables|Default|GetCurZ) (* DeltaSeconds (Variables|Default|GetDirection)))))
    (bind _asabp_boss (Utilities|Casting|CastToABP_Boss (Components|SkeletalMesh|GetAnimInstance (Variables|Character|GetMesh))))
    (Variables|/Game/EndlessGraves/AI/Boss/ABP_Boss.ABP_Boss_C|SetZRotation _asabp_boss _output_get)
    (if (<= (Variables|Default|GetCurZ) (Variables|Default|GetMinZ))
      (Variables|Default|SetDirection 1.0)
      (elif (>= (Variables|Default|GetCurZ) (Variables|Default|GetMaxZ))
        (Variables|Default|SetDirection -1.0)))))

(fn ConstructionScript)

(fn GetRotationAroundZ
  (bind _returnvalue (Class|EndlessGravesBossCharacter|GetRotationZ))
  (return _returnvalue))