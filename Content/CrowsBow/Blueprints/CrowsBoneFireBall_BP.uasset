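; CrowsBoneFireBall_BP is a fireball effect actor in the CrowsBow content.
; Its ActiveParticle event switches the particle system on or off from a State input, without resetting it.
; An unconnected node chain would billboard the actor toward the player camera with a 90-degree pitch offset, but it never runs.
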(event EventActiveParticle
  (params (state :type Boolean))
  (Components|Activation|SetActive (Variables|Default|GetParticleSystem) state false))

(fn ConstructionScript)