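; Player character for CrowsBow that starts with input disabled and the mouse cursor shown.
; It emits noise every tick for pawn sensing and forwards capsule overlaps to an OnBeginOverlap handler.
; GameOver disables input, shows the cursor and adds the GameOver widget to the viewport.
; OnSlashSword plays the slash montage unless it is already playing.
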(event OnComponentBeginOverlap(CapsuleComponent)
  (params (OverlappedComponent :type Primitive%20Component%20Object%20Reference) (OtherActor :type Actor%20Object%20Reference) (OtherComp :type Primitive%20Component%20Object%20Reference) (OtherBodyIndex :type Integer) (bFromSweep :type Boolean) (SweepResult :type Hit%20Result%20Structure%20%28by%20ref%29))
  (Class|CrowsBowCharacter|OnBeginOverlap OverlappedComponent OtherActor OtherComp OtherBodyIndex bFromSweep SweepResult))

(event EventBeginPlay
  (bind _returnvalue (Game|GetPlayerController 0))
  (Input|DisableInput _returnvalue)
  (Variables|/Script/Engine.PlayerController|SetbShowMouseCursor _returnvalue true))

(event Collision|EventActorBeginOverlap
  (params (OtherActor :type Actor%20Object%20Reference)))

(event EventTick
  (params (DeltaSeconds :type Float%20%28single-precision%29))
  (Class|Pawn|PawnMakeNoise 1.0 "0, 0, 0" true self))

(event EventGameOver
  (bind _returnvalue (Game|GetPlayerController 0))
  (Input|DisableInput _returnvalue)
  (Variables|/Script/Engine.PlayerController|SetbShowMouseCursor _returnvalue true)
  (bind _returnvalue_2 (UserInterface|CreateWidget "/Game/CrowsBow/UI/GameOver_BP.GameOver_BP_C" _returnvalue))
  (UserInterface|Viewport|AddtoViewport _returnvalue_2 0))

(event EventOnSlashSword
  (if (not (Animation|Montage|MontageIsPlaying (Components|SkeletalMesh|GetAnimInstance (Variables|Character|GetMesh)) "/Game/CrowAnimations/Slash1_0_Montage.Slash1_0_Montage"))
    (Animation|PlayAnimMontage "/Game/CrowAnimations/Slash1_0_Montage.Slash1_0_Montage" 1.6 "None")))

(fn ConstructionScript)