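; Double door actor that the player can open and close when standing in a front or back trigger and the doors are unlocked.
; Trigger overlaps set the interaction flags, and OpenDoors plays or reverses one timeline that swings both door arrows in mirrored yaw.
; DoOnce gates block repeat input until the animation finishes and flips DoorsOpen.
; The construction script sets the initial open pose and hides the back archway for one-sided doors.
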(event OnComponentBeginOverlap(Doors_Front_Trigger)
  (params (OverlappedComponent :type Primitive%20Component%20Object%20Reference) (OtherActor :type Actor%20Object%20Reference) (OtherComp :type Primitive%20Component%20Object%20Reference) (OtherBodyIndex :type Integer) (bFromSweep :type Boolean) (SweepResult :type Hit%20Result%20Structure%20%28by%20ref%29))
  (CallFunction|ActivateDoors OtherActor))

(event OnComponentEndOverlap(Doors_Front_Trigger)
  (params (OverlappedComponent :type Primitive%20Component%20Object%20Reference) (OtherActor :type Actor%20Object%20Reference) (OtherComp :type Primitive%20Component%20Object%20Reference) (OtherBodyIndex :type Integer))
  (CallFunction|DeactivateDoors OtherActor))

(event OnComponentBeginOverlap(Doors_Back_Trigger)
  (params (OverlappedComponent :type Primitive%20Component%20Object%20Reference) (OtherActor :type Actor%20Object%20Reference) (OtherComp :type Primitive%20Component%20Object%20Reference) (OtherBodyIndex :type Integer) (bFromSweep :type Boolean) (SweepResult :type Hit%20Result%20Structure%20%28by%20ref%29))
  (CallFunction|ActivateDoors OtherActor))

(event OnComponentEndOverlap(Doors_Back_Trigger)
  (params (OverlappedComponent :type Primitive%20Component%20Object%20Reference) (OtherActor :type Actor%20Object%20Reference) (OtherComp :type Primitive%20Component%20Object%20Reference) (OtherBodyIndex :type Integer))
  (CallFunction|DeactivateDoors OtherActor))

(event Custom|DeactivateDoors
  (params (Other%20Actor :type Actor%20Object%20Reference))
  (if (== Other%20Actor (Game|GetPlayerCharacter 0))
    (Variables|Default|SetactiveDoors false :!label _label)
    (Variables|Default|SetcanInteractDoors false)
    (elif (or (== Other%20Actor (Variables|Default|GetLeft%20Door)) (== Other%20Actor (Variables|Default|GetRight%20Door)))
      (goto _label))))

(event Custom|Open%20Doors
  (if (not (Variables|Default|GetDoorsLocked))
    (if (Variables|Default|GetcanInteractDoors)
      (if (not (Variables|Default|GetDoorsOpen))
        (Utilities|FlowControl|DoOnce false
          (:Completed
            (bind _doorsangle (Timeline|DoorAnimation PlayFromStart)
              (:Update
                (Transformation|SetRelativeRotation (Variables|Default|GetLeft%20Door%20Arrow) (Math|Rotator|MakeRotator 0.0 0.0 _doorsangle) false false)
                (Transformation|SetRelativeRotation (Variables|Default|GetRight%20Door%20Arrow) (Math|Rotator|MakeRotator 0.0 0.0 (- 1.8e+02 _doorsangle)) false false))
              (:Finished
                (if (Variables|Default|GetDoorsOpen)
                  (Variables|Default|SetDoorsOpen false)
                  (else
                    (Variables|Default|SetDoorsOpen true)))
                (CallFunction|ResetDoors)))))
        (else
          (Utilities|FlowControl|DoOnce false
            (:Completed
              (Timeline|DoorAnimation ReverseFromEnd))))))))

(event Custom|ActivateDoors
  (params (Other%20Actor :type Actor%20Object%20Reference))
  (if (== Other%20Actor (Game|GetPlayerCharacter 0))
    (Variables|Default|SetactiveDoors true :!label _label)
    (Variables|Default|SetcanInteractDoors true)
    (elif (or (== Other%20Actor (Variables|Default|GetLeft%20Door)) (== Other%20Actor (Variables|Default|GetRight%20Door)))
      (goto _label))))

(event Custom|ResetDoors
  (Utilities|FlowControl|Sequence
    (:then_0
      (Utilities|FlowControl|DoOnce false) ; enters at Reset
    )
    (:then_1
      (Utilities|FlowControl|DoOnce false) ; enters at Reset
    )))

(event EventBeginPlay
  (Variables|Default|SetcanInteractDoors false)
  (Collision|IgnoreActorwhenMoving (Variables|Default|GetLeft%20Door) (Game|GetPlayerCharacter 0) true))

(fn ConstructionScript
  (bind _left_door_arrow (Variables|Default|GetLeft%20Door%20Arrow))
  (bind _right_door_arrow (Variables|Default|GetRight%20Door%20Arrow))
  (bind _wall_archway_back (Variables|Default|GetWall_Archway_Back))
  (Utilities|FlowControl|Sequence
    (:then_0
      (if (Variables|Default|GetOneSided)
        (Rendering|SetVisibility _wall_archway_back false false)
        (else
          (Rendering|SetVisibility _wall_archway_back true false))))
    (:then_1
      (if (Variables|Default|GetDoorsOpen)
        (Transformation|SetRelativeRotation _left_door_arrow "0,90.000000, 0" false false)
        (Transformation|SetRelativeRotation _right_door_arrow "0,90.000000, 0" false false)
        (else
          (Transformation|SetRelativeRotation _left_door_arrow "0, 0, 0" false false)
          (Transformation|SetRelativeRotation _right_door_arrow "0,180.000000, 0" false false))))))