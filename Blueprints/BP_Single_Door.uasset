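; Single swinging door actor that the player can open and close while inside a front or back trigger, unless it is locked.
; OpenDoor, not called within this Blueprint, plays or reverses a timeline that yaws DoorArrow, optionally inverted.
; DoOnce gates block retriggering until the timeline finishes and toggles DoorOpen.
; The construction script sets back archway visibility, initial door rotation and the open-direction indicator.
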(event OnComponentBeginOverlap(Door_Front_Trigger)
  (params (OverlappedComponent :type Primitive%20Component%20Object%20Reference) (OtherActor :type Actor%20Object%20Reference) (OtherComp :type Primitive%20Component%20Object%20Reference) (OtherBodyIndex :type Integer) (bFromSweep :type Boolean) (SweepResult :type Hit%20Result%20Structure%20%28by%20ref%29))
  (CallFunction|ActivateDoor OtherActor))

(event OnComponentEndOverlap(Door_Front_Trigger)
  (params (OverlappedComponent :type Primitive%20Component%20Object%20Reference) (OtherActor :type Actor%20Object%20Reference) (OtherComp :type Primitive%20Component%20Object%20Reference) (OtherBodyIndex :type Integer))
  (CallFunction|DeactivateDoor OtherActor))

(event OnComponentBeginOverlap(Door_Back_Trigger)
  (params (OverlappedComponent :type Primitive%20Component%20Object%20Reference) (OtherActor :type Actor%20Object%20Reference) (OtherComp :type Primitive%20Component%20Object%20Reference) (OtherBodyIndex :type Integer) (bFromSweep :type Boolean) (SweepResult :type Hit%20Result%20Structure%20%28by%20ref%29))
  (CallFunction|ActivateDoor OtherActor))

(event OnComponentEndOverlap(Door_Back_Trigger)
  (params (OverlappedComponent :type Primitive%20Component%20Object%20Reference) (OtherActor :type Actor%20Object%20Reference) (OtherComp :type Primitive%20Component%20Object%20Reference) (OtherBodyIndex :type Integer))
  (CallFunction|DeactivateDoor OtherActor))

(event Custom|DeactivateDoor
  (params (Other%20Actor :type Actor%20Object%20Reference))
  (if (== Other%20Actor (Game|GetPlayerCharacter 0))
    (Variables|Default|SetactiveDoor false :!label _label)
    (Variables|Default|SetcanInteractDoor false)
    (elif (== Other%20Actor (Variables|Default|GetDoor))
      (goto _label))))

(event Custom|Open%20Door
  (bind _door_arrow (Variables|Default|GetDoor%20Arrow))
  (if (not (Variables|Default|GetDoorLocked))
    (if (Variables|Default|GetcanInteractDoor)
      (if (not (Variables|Default|GetDoorOpen))
        (Utilities|FlowControl|DoOnce false
          (:Completed
            (bind _doorangle (Timeline|DoorAnimation2 PlayFromStart)
              (:Update
                (if (Variables|Default|GetInvertOpen%20Direction)
                  (Transformation|SetRelativeRotation _door_arrow (Math|Rotator|MakeRotator 0.0 0.0 (* _doorangle -1.0)) false false)
                  (else
                    (Transformation|SetRelativeRotation _door_arrow (Math|Rotator|MakeRotator 0.0 0.0 _doorangle) false false))))
              (:Finished
                (if (Variables|Default|GetDoorOpen)
                  (Variables|Default|SetDoorOpen false)
                  (else
                    (Variables|Default|SetDoorOpen true)))
                (CallFunction|ResetDoor)))))
        (else
          (Utilities|FlowControl|DoOnce false
            (:Completed
              (Timeline|DoorAnimation2 ReverseFromEnd))))))))

(event Custom|ActivateDoor
  (params (Other%20Actor :type Actor%20Object%20Reference))
  (if (== Other%20Actor (Game|GetPlayerCharacter 0))
    (Variables|Default|SetactiveDoor true :!label _label)
    (Variables|Default|SetcanInteractDoor true)
    (elif (== Other%20Actor (Variables|Default|GetDoor))
      (goto _label))))

(event Custom|ResetDoor
  (bind _door_arrow (Variables|Default|GetDoor%20Arrow))
  (Utilities|FlowControl|Sequence
    (:then_0
      (Utilities|FlowControl|DoOnce false) ; enters at Reset
    )
    (:then_1
      (Utilities|FlowControl|DoOnce false) ; enters at Reset
    )))

(event EventBeginPlay
  (Variables|Default|SetcanInteractDoor false)
  (Collision|IgnoreActorwhenMoving (Variables|Default|GetDoor) (Game|GetPlayerCharacter 0) true))

(fn ConstructionScript
  (bind _door_arrow (Variables|Default|GetDoor%20Arrow))
  (bind _wall_archway_back (Variables|Default|GetWall_Archway_Back))
  (bind _open_direction (Variables|Default|GetOpen%20Direction))
  (Utilities|FlowControl|Sequence
    (:then_0
      (if (Variables|Default|GetOneSided)
        (Rendering|SetVisibility _wall_archway_back false false)
        (else
          (Rendering|SetVisibility _wall_archway_back true false))))
    (:then_1
      (if (Variables|Default|GetDoorOpen)
        (Transformation|SetRelativeRotation _door_arrow "0,110.000000, 0" false false)
        (else
          (Transformation|SetRelativeRotation _door_arrow "0, 0, 0" false false))))
    (:then_2
      (if (Variables|Default|GetInvertOpen%20Direction)
        (Transformation|SetRelativeRotation _open_direction "0,-90.000000, 0" false false)
        (else
          (Transformation|SetRelativeRotation _open_direction "0,90.000000, 0" false false))))))