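; Portcullis gate actor that the player can raise and lower while standing in its front or back trigger.
; Trigger overlaps by the player toggle the interaction flags, and OpenGate, not called within this graph, checks them and the lock.
; A timeline slides the gate vertically, flipping GateOpen on finish, with DoOnce nodes blocking re-triggering mid-animation.
; The construction script previews the open state and hides the back archway for one-sided gates.
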(event OnComponentBeginOverlap(Door_Front_Trigger)
  (params (OverlappedComponent :type Primitive%20Component%20Object%20Reference) (OtherActor :type Actor%20Object%20Reference) (OtherComp :type Primitive%20Component%20Object%20Reference) (OtherBodyIndex :type Integer) (bFromSweep :type Boolean) (SweepResult :type Hit%20Result%20Structure%20%28by%20ref%29))
  (CallFunction|ActivateGate OtherActor))

(event OnComponentEndOverlap(Door_Front_Trigger)
  (params (OverlappedComponent :type Primitive%20Component%20Object%20Reference) (OtherActor :type Actor%20Object%20Reference) (OtherComp :type Primitive%20Component%20Object%20Reference) (OtherBodyIndex :type Integer))
  (CallFunction|DeactivateGate OtherActor))

(event OnComponentBeginOverlap(Door_Back_Trigger)
  (params (OverlappedComponent :type Primitive%20Component%20Object%20Reference) (OtherActor :type Actor%20Object%20Reference) (OtherComp :type Primitive%20Component%20Object%20Reference) (OtherBodyIndex :type Integer) (bFromSweep :type Boolean) (SweepResult :type Hit%20Result%20Structure%20%28by%20ref%29))
  (CallFunction|ActivateGate OtherActor))

(event OnComponentEndOverlap(Door_Back_Trigger)
  (params (OverlappedComponent :type Primitive%20Component%20Object%20Reference) (OtherActor :type Actor%20Object%20Reference) (OtherComp :type Primitive%20Component%20Object%20Reference) (OtherBodyIndex :type Integer))
  (CallFunction|DeactivateGate OtherActor))

(event Custom|DeactivateGate
  (params (Other%20Actor :type Actor%20Object%20Reference))
  (if (== Other%20Actor (Game|GetPlayerCharacter 0))
    (Variables|Default|SetactiveGate false)
    (Variables|Default|SetcanInteractGate false)))

(event Custom|Open%20Gate
  (if (not (Variables|Default|GetGateLocked))
    (if (Variables|Default|GetcanInteractGate)
      (if (not (Variables|Default|GetGateOpen))
        (Utilities|FlowControl|DoOnce false
          (:Completed
            (bind _gateheight (Timeline|GateAnimation PlayFromStart)
              (:Update
                (Transformation|SetRelativeLocation (Variables|Default|GetPortculis) (Math|Vector|MakeVector 2.5e+02 0.0 _gateheight) false false))
              (:Finished
                (if (Variables|Default|GetGateOpen)
                  (Variables|Default|SetGateOpen false)
                  (else
                    (Variables|Default|SetGateOpen true)))
                (CallFunction|ResetGate)))))
        (else
          (Utilities|FlowControl|DoOnce false
            (:Completed
              (Timeline|GateAnimation ReverseFromEnd))))))))

(event Custom|ActivateGate
  (params (Other%20Actor :type Actor%20Object%20Reference))
  (if (== Other%20Actor (Game|GetPlayerCharacter 0))
    (Variables|Default|SetactiveGate true)
    (Variables|Default|SetcanInteractGate true)))

(event Custom|ResetGate
  (Utilities|FlowControl|Sequence
    (:then_0
      (Utilities|FlowControl|DoOnce false) ; enters at Reset
    )
    (:then_1
      (Utilities|FlowControl|DoOnce false) ; enters at Reset
    )))

(event EventBeginPlay
  (Variables|Default|SetcanInteractGate false))

(fn ConstructionScript
  (bind _wall_archway_back (Variables|Default|GetWall_Archway_Back))
  (bind _portculis (Variables|Default|GetPortculis))
  (Utilities|FlowControl|Sequence
    (:then_0
      (if (Variables|Default|GetOneSided)
        (Rendering|SetVisibility _wall_archway_back false false)
        (else
          (Rendering|SetVisibility _wall_archway_back true false))))
    (:then_1
      (if (Variables|Default|GetGateOpen)
        (Transformation|SetRelativeLocation _portculis "250.000000, 0,200.000000" false false)
        (else
          (Transformation|SetRelativeLocation _portculis "250.000000, 0, 0" false false))))))