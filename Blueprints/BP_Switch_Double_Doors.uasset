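; A lever switch that unlocks and opens a referenced set of double doors, usable once.
; Overlap on the collision box enables interaction only while the player character is inside.
; UseLever plays a wall or standing timeline to rotate the handle, then OperateDoor unlocks and opens DoorToOperate.
; The construction script arranges the collision box for wall or left/right side use, and presets the handle rotation when wall-mounted.
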(event OnComponentBeginOverlap(LeverCollisionBox)
  (params (OverlappedComponent :type Primitive%20Component%20Object%20Reference) (OtherActor :type Actor%20Object%20Reference) (OtherComp :type Primitive%20Component%20Object%20Reference) (OtherBodyIndex :type Integer) (bFromSweep :type Boolean) (SweepResult :type Hit%20Result%20Structure%20%28by%20ref%29))
  (CallFunction|ActivateLever OtherActor))

(event OnComponentEndOverlap(LeverCollisionBox)
  (params (OverlappedComponent :type Primitive%20Component%20Object%20Reference) (OtherActor :type Actor%20Object%20Reference) (OtherComp :type Primitive%20Component%20Object%20Reference) (OtherBodyIndex :type Integer))
  (CallFunction|DeactivateLever OtherActor))

(event Custom|UseLever
  (if (Variables|Default|GetCan%20Interact%20Lever)
    (Utilities|FlowControl|DoOnce false
      (:Completed
        (if (Variables|Default|GetplacedOnWall)
          (bind _rotation (Timeline|Lever_movement_Wall PlayFromStart)
            (:Update
              (Transformation|SetRelativeRotation (Variables|Default|GetLever_Handle) (Math|Rotator|MakeRotator _rotation 0.0 0.0) false false))
            (:Finished
              (CallFunction|OperateDoor)))
          (else
            (bind _rotation_2 (Timeline|Lever_Movement PlayFromStart)
              (:Update
                (Transformation|SetRelativeRotation (Variables|Default|GetLever_Handle) (Math|Rotator|MakeRotator _rotation_2 0.0 0.0) false false))
              (:Finished
                (CallFunction|OperateDoor)))))))))

(event Custom|Operate%20Door
  (bind _door_to_operate (Variables|Default|GetDoor%20to%20operate))
  (Variables|/Game/HG_Poly/Medieval/Catacombs/Blueprints/BP_Double_Doors.BP_Double_Doors_C|SetcanInteractDoors _door_to_operate true)
  (Variables|/Game/HG_Poly/Medieval/Catacombs/Blueprints/BP_Double_Doors.BP_Double_Doors_C|SetDoorsLocked _door_to_operate false)
  (Default|OpenDoors _door_to_operate))

(event Custom|Deactivate%20Lever
  (params (Other%20Actor :type Actor%20Object%20Reference))
  (if (== Other%20Actor (Game|GetPlayerCharacter 0))
    (Variables|Default|SetActive%20Lever false)
    (Variables|Default|SetCan%20Interact%20Lever false)))

(event Custom|Activate%20Lever
  (params (Other%20Actor :type Actor%20Object%20Reference))
  (if (== Other%20Actor (Game|GetPlayerCharacter 0))
    (Variables|Default|SetActive%20Lever true)
    (Variables|Default|SetCan%20Interact%20Lever true)))

(fn ConstructionScript
  (bind _levercollisionbox (Variables|Default|GetLeverCollisionBox))
  (if (Variables|Default|GetplacedOnWall)
    (Transformation|SetRelativeTransform (Variables|Default|GetLeverCollisionBox) (Math|Transform|MakeTransform "0, 0,94.000000" "0, 0, 0" "2.000000,2.000000,2.000000") false false)
    (Transformation|SetRelativeRotation (Variables|Default|GetLever_Handle) "0,0.000000,-75.000000" false false)
    (else
      (Transformation|SetRelativeScale3D (Variables|Default|GetLeverCollisionBox) "1.000000,1.000000,1.000000")
      (switch Utilities|FlowControl|Switch|SwitchonE_Use_Side (Variables|Default|GetUse%20Side)
        (:NewEnumerator0
          (Transformation|SetRelativeLocation _levercollisionbox "-32.000000, 0,50.000000" false false))
        (:NewEnumerator1
          (Transformation|SetRelativeLocation _levercollisionbox "32.000000, 0,50.000000" false false))))))