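; Interactable chest whose lid toggles open and closed while the player character is in range.
; InteractRange overlaps set ActiveChest and CanInteractChest, and the OpenChest event acts only when interaction is allowed.
; A timeline drives lid roll, playing forward or in reverse according to LidOpen.
; DoOnce gates block repeat triggers until the timeline finishes, flips LidOpen and calls ResetChest.
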(event OnComponentBeginOverlap(InteractRange)
  (params (OverlappedComponent :type Primitive%20Component%20Object%20Reference) (OtherActor :type Actor%20Object%20Reference) (OtherComp :type Primitive%20Component%20Object%20Reference) (OtherBodyIndex :type Integer) (bFromSweep :type Boolean) (SweepResult :type Hit%20Result%20Structure%20%28by%20ref%29))
  (if (== OtherActor (Game|GetPlayerCharacter 0))
    (Variables|Default|SetactiveChest true)
    (Variables|Default|SetcanInteractChest true)
    (else
      (Development|PrintString "Not player pawn"))))

(event OnComponentEndOverlap(InteractRange)
  (params (OverlappedComponent :type Primitive%20Component%20Object%20Reference) (OtherActor :type Actor%20Object%20Reference) (OtherComp :type Primitive%20Component%20Object%20Reference) (OtherBodyIndex :type Integer))
  (if (== OtherActor (Game|GetPlayerCharacter 0))
    (Variables|Default|SetactiveChest false)
    (Variables|Default|SetcanInteractChest false)))

(event Custom|OpenChest
  (if (Variables|Default|GetcanInteractChest)
    (if (not (Variables|Default|GetlidOpen))
      (Utilities|FlowControl|DoOnce false
        (:Completed
          (bind _time (Timeline|Timeline_0 PlayFromStart)
            (:Update
              (Transformation|SetRelativeRotation (Variables|Default|GetChest_Lid) (Math|Rotator|MakeRotator _time 0.0 0.0) false false))
            (:Finished
              (if (Variables|Default|GetlidOpen)
                (Variables|Default|SetlidOpen false)
                (else
                  (Variables|Default|SetlidOpen true)))
              (CallFunction|ResetChest)))))
      (else
        (Utilities|FlowControl|DoOnce false
          (:Completed
            (Timeline|Timeline_0 ReverseFromEnd)))))))

(event Custom|ResetChest
  (Utilities|FlowControl|Sequence
    (:then_0
      (Utilities|FlowControl|DoOnce false) ; enters at Reset
    )
    (:then_1
      (Utilities|FlowControl|DoOnce false) ; enters at Reset
    )))

(event EventBeginPlay
  (Variables|Default|SetcanInteractChest false))

(event Collision|EventActorBeginOverlap
  (params (OtherActor :type Actor%20Object%20Reference)))

(event EventTick
  (params (DeltaSeconds :type Float%20%28single-precision%29)))

(fn ConstructionScript)