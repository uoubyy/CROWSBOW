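; Interactable vase with six body types and a lid that opens and closes.
; The construction script sets the body and lid meshes, their yaw and the Arrow pivot position per type.
; Sphere overlap lets OpenVase work only while the player is in range.
; OpenVase toggles by playing or reversing a DoOnce-guarded timeline that yaws the Arrow left or right, at half angle for types 4 and 5.
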(event OnComponentBeginOverlap(VaseSphereCollision)
  (params (OverlappedComponent :type Primitive%20Component%20Object%20Reference) (OtherActor :type Actor%20Object%20Reference) (OtherComp :type Primitive%20Component%20Object%20Reference) (OtherBodyIndex :type Integer) (bFromSweep :type Boolean) (SweepResult :type Hit%20Result%20Structure%20%28by%20ref%29))
  (CallFunction|ActivateVase OtherActor))

(event OnComponentEndOverlap(VaseSphereCollision)
  (params (OverlappedComponent :type Primitive%20Component%20Object%20Reference) (OtherActor :type Actor%20Object%20Reference) (OtherComp :type Primitive%20Component%20Object%20Reference) (OtherBodyIndex :type Integer))
  (CallFunction|DeactivateVase OtherActor))

(event Custom|Deactivate%20Vase
  (params (Other%20Actor :type Actor%20Object%20Reference))
  (if (== Other%20Actor (Game|GetPlayerCharacter 0))
    (Variables|Default|SetactiveVase false)
    (Variables|Default|SetcanIntractVase false)))

(event Custom|Activate%20Vase
  (params (Other%20Actor :type Actor%20Object%20Reference))
  (if (== Other%20Actor (Game|GetPlayerCharacter 0))
    (Variables|Default|SetactiveVase true)
    (Variables|Default|SetcanIntractVase true)))

(event Custom|Open%20Vase
  (bind _arrow (Variables|Default|GetArrow))
  (if (Variables|Default|GetcanIntractVase)
    (if (not (Variables|Default|GetvaseOpen))
      (Utilities|FlowControl|DoOnce false
        (:Completed
          (bind _lidrotation (Timeline|VaseLidMove PlayFromStart)
            (:Update
              (switch Utilities|FlowControl|Switch|SwitchonE_OpenDirection (Variables|Default|GetLid%20Open%20Direction)
                (:NewEnumerator0
                  (switch Utilities|FlowControl|Switch|SwitchonE_Vases_Body_Types (Variables|Default|GetVase%20Type)
                    (:NewEnumerator0
                      (Transformation|SetRelativeRotation _arrow (Math|Rotator|MakeRotator 0.0 0.0 (- 9e+01 _lidrotation)) false false :!label _label))
                    (:NewEnumerator1
                      (goto _label))
                    (:NewEnumerator2
                      (goto _label))
                    (:NewEnumerator3
                      (Transformation|SetRelativeRotation _arrow (Math|Rotator|MakeRotator 0.0 0.0 (- 9e+01 (/ _lidrotation 2.0))) false false :!label _label_2))
                    (:NewEnumerator4
                      (goto _label_2))
                    (:NewEnumerator5
                      (goto _label))))
                (:NewEnumerator1
                  (switch Utilities|FlowControl|Switch|SwitchonE_Vases_Body_Types (Variables|Default|GetVase%20Type)
                    (:NewEnumerator0
                      (Transformation|SetRelativeRotation _arrow (Math|Rotator|MakeRotator 0.0 0.0 (+ 9e+01 _lidrotation)) false false :!label _label_3))
                    (:NewEnumerator1
                      (goto _label_3))
                    (:NewEnumerator2
                      (goto _label_3))
                    (:NewEnumerator3
                      (Transformation|SetRelativeRotation _arrow (Math|Rotator|MakeRotator 0.0 0.0 (+ 9e+01 (/ _lidrotation 2.0))) false false :!label _label_4))
                    (:NewEnumerator4
                      (goto _label_4))
                    (:NewEnumerator5
                      (goto _label_3))))))
            (:Finished
              (if (Variables|Default|GetvaseOpen)
                (Variables|Default|SetvaseOpen false)
                (else
                  (Variables|Default|SetvaseOpen true)))
              (CallFunction|ResetVase)))))
      (else
        (Utilities|FlowControl|DoOnce false
          (:Completed
            (Timeline|VaseLidMove ReverseFromEnd)))))))

(event Custom|Reset%20Vase
  (bind _arrow (Variables|Default|GetArrow))
  (Utilities|FlowControl|Sequence
    (:then_0
      (Utilities|FlowControl|DoOnce false) ; enters at Reset
    )
    (:then_1
      (Utilities|FlowControl|DoOnce false) ; enters at Reset
    )))

(fn ConstructionScript
  (bind _vase_type (Variables|Default|GetVase%20Type))
  (bind _arrow (Variables|Default|GetArrow))
  (bind _returnvalue (Utilities|Select :Index _vase_type :NewEnumerator0 0 :NewEnumerator1 1 :NewEnumerator2 2 :NewEnumerator3 3 :NewEnumerator4 4 :NewEnumerator5 5))
  (Utilities|FlowControl|Sequence
    (:then_0
      (Components|StaticMesh|SetStaticMesh (Variables|Default|GetVase_Body) (Utilities|Array|Get(acopy) (Variables|Default|GetVasesBodies) _returnvalue)))
    (:then_1
      (Components|StaticMesh|SetStaticMesh (Variables|Default|GetVase_Lid) (Utilities|Array|Get(acopy) (Variables|Default|GetVasesLids) _returnvalue)))
    (:then_2
      (Transformation|SetRelativeRotation (Variables|Default|GetVase_Body) (Math|Rotator|MakeRotator 0.0 0.0 (Variables|Default|GetVaseRotation)) false false)
      (switch Utilities|FlowControl|Switch|SwitchonE_Vases_Body_Types (Variables|Default|GetVase%20Type)
        (:NewEnumerator0
          (Transformation|SetRelativeLocation _arrow "0.000000,-20.000000,93.000000" false false :!label _label))
        (:NewEnumerator1
          (goto _label))
        (:NewEnumerator2
          (Transformation|SetRelativeLocation _arrow "0.000000,-20.000000,56.000000" false false))
        (:NewEnumerator3
          (goto _label))
        (:NewEnumerator4
          (Transformation|SetRelativeLocation _arrow "0.000000,-20.000000,40.000000" false false :!label _label_2))
        (:NewEnumerator5
          (goto _label_2))))))