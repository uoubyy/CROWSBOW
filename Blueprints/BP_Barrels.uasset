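; BP_Barrels is an interactive barrel actor whose lid can be opened and closed while the player character is inside its collision sphere.
; OpenBarrel plays or reverses a timeline that yaws an Arrow component left or right per LidOpenDirection, toggling BarrelOpen on finish.
; DoOnce gates, reset when the timeline finishes, block retriggering mid-animation.
; The construction script picks body and lid meshes from type settings and applies a configurable rotation.
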(event OnComponentBeginOverlap(BarrelSphereCollision)
  (params (OverlappedComponent :type Primitive%20Component%20Object%20Reference) (OtherActor :type Actor%20Object%20Reference) (OtherComp :type Primitive%20Component%20Object%20Reference) (OtherBodyIndex :type Integer) (bFromSweep :type Boolean) (SweepResult :type Hit%20Result%20Structure%20%28by%20ref%29))
  (CallFunction|ActivateBarrel OtherActor))

(event OnComponentEndOverlap(BarrelSphereCollision)
  (params (OverlappedComponent :type Primitive%20Component%20Object%20Reference) (OtherActor :type Actor%20Object%20Reference) (OtherComp :type Primitive%20Component%20Object%20Reference) (OtherBodyIndex :type Integer))
  (CallFunction|DeactivateBarrel OtherActor))

(event Custom|Deactivate%20Barrel
  (params (Other%20Actor :type Actor%20Object%20Reference))
  (if (== Other%20Actor (Game|GetPlayerCharacter 0))
    (Variables|Default|SetactiveBarrel false)
    (Variables|Default|SetcanIntractBarrel false)))

(event Custom|Activate%20Barrel
  (params (Other%20Actor :type Actor%20Object%20Reference))
  (if (== Other%20Actor (Game|GetPlayerCharacter 0))
    (Variables|Default|SetactiveBarrel true)
    (Variables|Default|SetcanIntractBarrel true)))

(event Custom|Open%20Barrel
  (bind _arrow (Variables|Default|GetArrow))
  (if (Variables|Default|GetcanIntractBarrel)
    (if (not (Variables|Default|GetbarrelOpen))
      (Utilities|FlowControl|DoOnce false
        (:Completed
          (bind _lidrotation (Timeline|BarrelLidMove PlayFromStart)
            (:Update
              (switch Utilities|FlowControl|Switch|SwitchonE_OpenDirection (Variables|Default|GetLid%20Open%20Direction)
                (:NewEnumerator0
                  (Transformation|SetRelativeRotation _arrow (Math|Rotator|MakeRotator 0.0 0.0 (- 9e+01 _lidrotation)) false false))
                (:NewEnumerator1
                  (Transformation|SetRelativeRotation _arrow (Math|Rotator|MakeRotator 0.0 0.0 (+ 9e+01 _lidrotation)) false false))))
            (:Finished
              (if (Variables|Default|GetbarrelOpen)
                (Variables|Default|SetbarrelOpen false)
                (else
                  (Variables|Default|SetbarrelOpen true)))
              (CallFunction|ResetBarrel)))))
      (else
        (Utilities|FlowControl|DoOnce false
          (:Completed
            (Timeline|BarrelLidMove ReverseFromEnd)))))))

(event Custom|Reset%20Barrel
  (bind _arrow (Variables|Default|GetArrow))
  (Utilities|FlowControl|Sequence
    (:then_0
      (Utilities|FlowControl|DoOnce false) ; enters at Reset
    )
    (:then_1
      (Utilities|FlowControl|DoOnce false) ; enters at Reset
    )))

(event EventBeginPlay)

(event Collision|EventActorBeginOverlap
  (params (OtherActor :type Actor%20Object%20Reference)))

(event EventTick
  (params (DeltaSeconds :type Float%20%28single-precision%29)))

(fn ConstructionScript
  (bind _barrel_body (Variables|Default|GetBarrel_Body))
  (bind _barrel_lid (Variables|Default|GetBarrel_Lid))
  (Utilities|FlowControl|Sequence
    (:then_0
      (switch Utilities|FlowControl|Switch|SwitchonE_Barrel_Body_Types (Variables|Default|GetBarrel%20Body%20Type)
        (:NewEnumerator0
          (Components|StaticMesh|SetStaticMesh _barrel_body "/Game/HG_Poly/Medieval/Catacombs/Meshes/Props/SM_Barrel_005_Body.SM_Barrel_005_Body"))
        (:NewEnumerator1
          (Components|StaticMesh|SetStaticMesh _barrel_body "/Game/HG_Poly/Medieval/Catacombs/Meshes/Props/SM_Barrel_006_Body.SM_Barrel_006_Body"))
        (:NewEnumerator2
          (Components|StaticMesh|SetStaticMesh _barrel_body "/Game/HG_Poly/Medieval/Catacombs/Meshes/Props/SM_Barrel_007_Body.SM_Barrel_007_Body"))))
    (:then_1
      (switch Utilities|FlowControl|Switch|SwitchonE_Barrel_Lid_Types (Variables|Default|GetBarrel%20Lid%20Type)
        (:NewEnumerator0
          (Components|StaticMesh|SetStaticMesh _barrel_lid "/Game/HG_Poly/Medieval/Catacombs/Meshes/Props/SM_Barrel_005_Lid.SM_Barrel_005_Lid"))
        (:NewEnumerator1
          (Components|StaticMesh|SetStaticMesh _barrel_lid "/Game/HG_Poly/Medieval/Catacombs/Meshes/Props/SM_Barrel_006_Lid.SM_Barrel_006_Lid"))
        (:NewEnumerator2
          (Components|StaticMesh|SetStaticMesh _barrel_lid "/Game/HG_Poly/Medieval/Catacombs/Meshes/Props/SM_Barrel_007_Lid.SM_Barrel_007_Lid"))))
    (:then_2
      (Transformation|SetRelativeRotation (Variables|Default|GetBarrel_Body) (Math|Rotator|MakeRotator 0.0 0.0 (Variables|Default|GetBarrelRotation)) false false))))